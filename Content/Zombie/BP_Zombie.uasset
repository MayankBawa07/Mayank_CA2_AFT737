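; BP_Zombie is a zombie enemy that takes damage and pays out a money reward when killed.
; On BeginPlay it reads walk speed and starting health from the DT_Zombie data table.
; AnyDamage subtracts health and also calls ApplyDamage on the instigator without setting an amount.
; At zero health or below, it finds BP_GameManager, adds the table's reward, reports the kill and destroys itself.
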(event EventBeginPlay
  (bind _returnvalue (Utilities|GetDataTableRow "/Game/Zombie/DT_Zombie.DT_Zombie" "Zombie")
    (:then
      (Variables|/Script/Engine.CharacterMovementComponent|SetMaxWalkSpeed (Variables|Character|GetCharacterMovement) (.Speed (Utilities|Struct|BreakST_Zombie _returnvalue)))
      (Variables|Default|SetCurrentHealth (.Health (Utilities|Struct|BreakST_Zombie _returnvalue))))))

(event Collision|EventActorBeginOverlap
  (params (OtherActor :type Actor%20Object%20Reference)))

(event Game|Damage|EventAnyDamage
  (params (Damage :type Float%20%28single-precision%29) (DamageType :type Damage%20Type%20Object%20Reference) (InstigatedBy :type Controller%20Object%20Reference) (DamageCauser :type Actor%20Object%20Reference))
  (Game|Damage|ApplyDamage InstigatedBy 0.0 0 DamageCauser)
  (bind _output_get (Variables|Default|SetCurrentHealth (- (Variables|Default|GetCurrentHealth) Damage)))
  (if (<= _output_get 0.0)
    (bind _outactors (Actor|GetAllActorsOfClass "/Game/BP_Coin/BP_GameManager.BP_GameManager_C"))
    (Utilities|IsValid (Utilities|Array|Get(acopy) _outactors)
      (:Is%20Valid
        (bind _returnvalue (Utilities|GetDataTableRow "/Game/Zombie/DT_Zombie.DT_Zombie" "Zombie")
          (:then
            (bind _asbp_game_manager (Utilities|Casting|CastToBP_GameManager (Utilities|Array|Get(acopy) _outactors)))
            (Default|AddMoney _asbp_game_manager (.Reward (Utilities|Struct|BreakST_Zombie _returnvalue)))
            (bind _outactors_2 (Actor|GetAllActorsOfClass "/Game/BP_Coin/BP_GameManager.BP_GameManager_C"))
            (bind _asbp_game_manager_2 (Utilities|Casting|CastToBP_GameManager (Utilities|Array|Get(acopy) _outactors_2)))
            (Default|OnZombieKilled _asbp_game_manager_2)
            (Actor|DestroyActor self)))))))

(event EventTick
  (params (DeltaSeconds :type Float%20%28single-precision%29)))

(fn ConstructionScript)