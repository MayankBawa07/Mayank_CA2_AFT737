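; Game manager actor for a zombie defense game that handles elixir money, cannon purchases and the win and lose screens.
; It creates the money widget on BeginPlay and updates it through AddMoney and SpendMoney.
; StartPlacingCannon pays the cost from a data table row, spawns a cannon and hands it to the top-down controller for placement.
; GameOver shows the loss widget, while OnZombieKilled shows Victory once kills reach the spawned total.
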(event Custom|GameOver
  (bind _returnvalue (UserInterface|CreateWidget "/Game/Game_Callouts/Game_Over.Game_Over_C"))
  (UserInterface|Viewport|AddtoViewport _returnvalue 0))

(event Custom|StartPlacingCannon
  (bind _returnvalue (Utilities|GetDataTableRow "/Game/BP_Cannon/DT_Cannon.DT_Cannon" "1")
    (:then
      (CallFunction|SpendMoney (.UpgradeCost (Utilities|Struct|BreakST_Cannon _returnvalue)))
      (if (Variables|Default|GetWasSuccessful)
        (bind _returnvalue_2 (Game|SpawnActorfromClass "/Game/BP_Cannon/BP_Cannon.BP_Cannon_C" (Transformation|GetActorTransform) "Undefined" "MultiplyWithRoot" 0 0 0))
        (bind _asbp_top_down_controller (Utilities|Casting|CastToBP_TopDownController (Game|GetPlayerController 0)))
        (Variables|/Game/TopDown/Blueprints/BP_TopDownController.BP_TopDownController_C|SetCannonBeingPlaced _asbp_top_down_controller _returnvalue_2)
        (Variables|/Game/TopDown/Blueprints/BP_TopDownController.BP_TopDownController_C|SetisPlacing _asbp_top_down_controller true)
        (else
          (Development|PrintString "Not ENough Money"))))))

(event Custom|OnZombieKilled
  (Variables|Default|SetTotalZombiesKilled (+ (Variables|Default|GetTotalZombiesKilled) 1))
  (if (>= (Variables|Default|GetTotalZombiesKilled) (Variables|Default|GetTotalZombiesSpawned))
    (bind _returnvalue (UserInterface|CreateWidget "/Game/Game_Callouts/Victory.Victory_C"))
    (UserInterface|Viewport|AddtoViewport _returnvalue 0)))

(event EventBeginPlay
  (bind _returnvalue (UserInterface|CreateWidget "/Game/BP_Elixir/Money_Widget.Money_Widget_C"))
  (bind _output_get (Variables|Default|SetWidget _returnvalue))
  (UserInterface|Viewport|AddtoViewport _output_get 0))

(event Collision|EventActorBeginOverlap
  (params (OtherActor :type Actor%20Object%20Reference)))

(fn ConstructionScript)

(fn AddMoney
  (params (Amount :type Integer))
  (bind _output_get (Variables|Default|SetElixir (+ (Variables|Default|GetPlayerMoney) Amount)))
  (Default|UpdateElixir (Variables|Default|GetWidget) _output_get)
  (Variables|Default|SetPlayerMoney (+ (Variables|Default|GetPlayerMoney) Amount)))

(fn SpendMoney
  (params (Cost :type Integer))
  (if (>= (Variables|Default|GetPlayerMoney) Cost)
    (Variables|Default|SetWasSuccessful true)
    (bind _output_get (Variables|Default|SetPlayerMoney (- (Variables|Default|GetPlayerMoney) Cost)))
    (Default|UpdateElixir (Variables|Default|GetWidget) _output_get)
    (else
      (Variables|Default|SetWasSuccessful false))))